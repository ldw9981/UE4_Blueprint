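; Destructible barrel actor that shows its HP on a text render and deals area damage when destroyed.
; Only radial damage lowers HP and refreshes the text, destroying the actor once HP reaches zero or below.
; The Destroyed event applies radial damage around the barrel, so nearby barrels can chain-react, then adds score through MyGameInstance.
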(event `self.ReceiveBeginPlay`
  (`TextRenderComponent.K2_SetText` (`self.TextRender`) (`KismetTextLibrary.Conv_DoubleToText` (`self.HP`) "HalfToEven")))

(event `self.ReceiveDestroyed`
  (`GameplayStatics.ApplyRadialDamage` :`BaseDamage` 10.0 :`Origin` (`self.K2_GetActorLocation`) :`DamageRadius` 100.0 :`DamageCauser` self :`InstigatedByController` null)
  (bind _asmy_game_instance (cast `/Game/Blueprints/MyGameInstance` (`GameplayStatics.GetGameInstance`)))
  (`/Game/Blueprints/MyGameInstance.AddScore` _asmy_game_instance 100))

(event `self.ReceiveRadialDamage`
  (params (DamageReceived :type "Float (single-precision)") (DamageType :type "DamageType Object Reference") (Origin :type "Vector Structure") (HitInfo :type "HitResult Structure (by ref)") (InstigatedBy :type "Controller Object Reference") (DamageCauser :type "Actor Object Reference"))
  (set `self.HP` (- (`self.HP`) DamageReceived))
  (`TextRenderComponent.K2_SetText` (`self.TextRender`) (`KismetTextLibrary.Conv_DoubleToText` (`self.HP`) "HalfToEven"))
  (if (<= (`self.HP`) 0.0)
    (`self.K2_DestroyActor`)))

(fn `UserConstructionScript`)