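; BP_StatusComponent is an actor component that holds HP, Defence and Damage stats, which can be filled from a monster struct.
; On BeginPlay it binds to the owner's OnTakeAnyDamage, ignores hits once dead, and otherwise subtracts raw damage from HP, clamped at zero.
; It then broadcasts OnChangeStatus, plus OnDeath when HP runs out.
; Defence and the damage causer's status component do not yet affect the calculation.
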(event `self.ReceiveBeginPlay`
  (add `Actor.OnTakeAnyDamage` (`self.GetOwner`) (delegate `OnTakeAnyDamage_Event_0`)))

(event `OnTakeAnyDamage_Event_0`
  (params (DamagedActor :type "Actor Object Reference") (Damage :type "Float (double-precision)") (DamageType :type "DamageType Object Reference") (InstigatedBy :type "Controller Object Reference") (DamageCauser :type "Actor Object Reference"))
  (bind _return (`self.IsDead`))
  (if (not _return)
    (`self.Take Damage` Damage (`Actor.GetComponentByClass` DamageCauser "BP_StatusComponent_C"))
    (`self.OnChangeStatus` InstigatedBy)
    (bind _return_2 (`self.IsDead`))
    (if _return_2
      (`self.OnDeath`))))

(fn `IsDead`
  (returns (Return :type Boolean))
  (return (<= (`self.HP`) 0.0)))

(fn `SetDataByMonsterStruct`
  (params (Monster :type "/Game/Blueprints/MonsterStruct Structure"))
  (set `self.HP` Monster_HP_5_9A9867B24AE507003960218173737F8A)
  (set `self.Defence` Monster_Defence_16_F17512AB44693345D28695BB62F6F475)
  (set `self.Damage` Monster_Damage_7_2469C997409F875E177C52801F949A3B))

(fn `Take Damage`
  (params (Value :type "Float (double-precision)") (OtherStatus :type "/Game/Blueprints/BP_StatusComponent Object Reference"))
  (set `self.HP` (`KismetMathLibrary.FMax` (- (`self.HP`) Value))))