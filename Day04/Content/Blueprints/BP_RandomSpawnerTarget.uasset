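; Spawner actor that places a randomly chosen actor class at the location of every TargetActorClass actor in the level on BeginPlay.
; With UseRespawn on, it binds to each spawned actor's OnDestroyed event and queues that actor's final location.
; A single shared Delay of RespawnDelay takes the oldest queued location and spawns a new random pick there, looping back to process queued requests one at a time.
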(event `self.ReceiveBeginPlay`
  (bind _actorclass (`self.ActorClass`))
  (bind _requestlocation (`self.RequestLocation`))
  (bind _outactors (`GameplayStatics.GetAllActorsOfClass` (`self.TargetActorClass`)))
  (for _array_element _outactors
    (set `self.SpawnLocation` (`self.K2_GetActorLocation` _array_element))
    (bind _returnvalue (`|SpawnActorFromClass` (`|GetArrayItem` _actorclass (`KismetMathLibrary.RandomInteger` (`KismetArrayLibrary.Array_Length` _actorclass))) (`KismetMathLibrary.MakeTransform` (`self.SpawnLocation`)) "Undefined" "OverrideRootScale" null null :!label _label))
    (`/Engine/EditorBlueprintResources/StandardMacros.IsValid` _returnvalue
      (:`Is Valid`
        (if (`self.UseRespawn`)
          (add `self.OnDestroyed` _returnvalue (delegate `OnDestroyed_Event_0`))
          (`KismetSystemLibrary.Delay` (`self.RespawnDelay`) :!label _label_2)
          (if (> (`KismetArrayLibrary.Array_Length` _requestlocation) 0)
            (set `self.SpawnLocation` (`|GetArrayItem` _requestlocation))
            (`KismetArrayLibrary.Array_Remove` _requestlocation)
            (goto _label)))))))

(event `OnDestroyed_Event_0` :!signature `self.OnDestroyed`
  (params (DestroyedActor :type "Actor Object Reference"))
  (`KismetArrayLibrary.Array_Add` (`self.RequestLocation`) (`self.K2_GetActorLocation` DestroyedActor))
  (goto _label_2))

(fn `UserConstructionScript`)