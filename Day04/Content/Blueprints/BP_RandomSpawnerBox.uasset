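; BP_RandomSpawnerBox spawns a set number of randomly chosen actor classes at random spots inside its box on BeginPlay.
; Each spot comes from a downward visibility trace with persistent debug drawing, and spawning happens only on a hit.
; With UseRespawn on, destroyed actors increment a waiting counter that one shared Delay drains, respawning one at a time by looping back to the trace.
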(event `self.ReceiveBeginPlay`
  (bind _actorclass (`self.ActorClass`))
  (bind _box (`self.Box`))
  (bind _returnvalue (`KismetMathLibrary.RandomPointInBoundingBox` (`SceneComponent.K2_GetComponentLocation` _box) (`BoxComponent.GetUnscaledBoxExtent` _box)))
  (for _ (range (`self.Number`))
    ;[1 1 1] Random 위치에 Random한 ActorClass  스폰
    (bind (_outhit _returnvalue_2) (`KismetSystemLibrary.LineTraceSingle` :`Start` _returnvalue :`End` (+ _returnvalue (0.0 0.0 -999.0)) :`TraceChannel` "TraceTypeQuery1" :`DrawDebugType` "Persistent" :!label _label))
    (if _returnvalue_2
      (bind _returnvalue_3 (`|SpawnActorFromClass` (`|GetArrayItem` _actorclass (`KismetMathLibrary.RandomInteger` (`KismetArrayLibrary.Array_Length` _actorclass))) (`KismetMathLibrary.MakeTransform` (`.Location` (`GameplayStatics.BreakHitResult` _outhit))) "AdjustIfPossibleButAlwaysSpawn" "OverrideRootScale" null null))
      (`/Engine/EditorBlueprintResources/StandardMacros.IsValid` _returnvalue_3
        (:`Is Valid`
          (if (`self.UseRespawn`)
            (add `self.OnDestroyed` _returnvalue_3 (delegate `OnDestroyed_Event_0`))
            ;[1 1 1] 딜레이가 끝나면 감소시키며  다시 스폰
            (`KismetSystemLibrary.Delay` (`self.RespawnDelayTime`) :!label _label_2)
            (if (> (`self.WaitingSpawnCount`) 0)
              (`/Engine/EditorBlueprintResources/StandardMacros.DecrementInt` (`self.WaitingSpawnCount`)
                (:`  `
                  (goto _label))))))))))

(event `OnDestroyed_Event_0` :!signature `self.OnDestroyed`
  (params (DestroyedActor :type "Actor Object Reference"))
  ;[1 1 1] 파괴된 이후에 WaitingSpawnCount 1증가하고 다시 딜레이스폰 시도 ( 딜레이중이면 스폰이 끝나고 다시 스폰시도됨)
  (`/Engine/EditorBlueprintResources/StandardMacros.IncrementInt` (`self.WaitingSpawnCount`)
    (:`  `
      (goto _label_2))))

(fn `UserConstructionScript`)