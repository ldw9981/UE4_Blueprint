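; BP_Zombie is an enemy that wanders around its spawn point, chases the player on sight or whoever damages it, and attacks in range.
; A Behavior enum, driven by Tick, PawnSensing and AIMoveTo results, switches states without a Behavior Tree.
; Animation notify messages time damage, attack exit and post-death destruction.
; Components supply data-table stats, status events and item drops, with name and HP shown as text.
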(event `self.ReceiveBeginPlay`
  (bind _returnvalue (`WidgetComponent.GetUserWidgetObject` (`self.Widget`)))
  (set `self.Start` (`self.K2_GetActorLocation`))
  (`/Engine/EditorBlueprintResources/StandardMacros.IsValid` _returnvalue
    (:`Is Valid`
      (bind _asstatus_widget (cast `/Game/Blueprints/StatusWidget` _returnvalue))
      (set `/Game/Blueprints/StatusWidget.StatusComponent` (`self.BP_StatusComponent`) _asstatus_widget))))

(event `self.ReceiveTick`
  (params (DeltaSeconds :type "Float (single-precision)"))
  (if (`|EnumEquality` (`self.Behavior`) "NewEnumerator0")
    (if (== (`KismetMathLibrary.VSize` (`MovementComponent.Velocity` (`self.CharacterMovement`))) 0.0)
      (`KismetSystemLibrary.Delay` (`KismetMathLibrary.RandomFloatInRange` 2.0 3.0))
      (if (`|EnumEquality` (`self.Behavior`) "NewEnumerator0")
        (cast `AIController` (`self.GetController`))
        (set `CharacterMovementComponent.MaxWalkSpeed` (`self.WalkSpeed`) (`self.CharacterMovement`))
        (`|AIMoveTo` self (`NavigationSystemV1.K2_GetRandomReachablePointInRadius` (`self.Start`) 500.0 null null) null)))))

(event `self.PawnSensing.OnSeePawn`
  (params (Pawn :type "Pawn Object Reference"))
  (bind _returnvalue (`GameplayStatics.GetPlayerPawn` 0))
  (if (`|EnumEquality` (`self.Behavior`) "NewEnumerator0")
    (if (== Pawn _returnvalue)
      (set `self.AttackTarget` _returnvalue)
      (set `self.Behavior` "NewEnumerator1" :!label _label)
      (set `CharacterMovementComponent.MaxWalkSpeed` (`self.RunSpeed`) (`self.CharacterMovement`))
      (`|AIMoveTo` self (0.0 0.0 0.0) (`self.AttackTarget`)
        (:`OnSuccess`
          (set `self.Behavior` "NewEnumerator2"))
        (:`OnFail`
          (set `self.Behavior` "NewEnumerator0"))))))

(event `self.BP_StatusComponent.OnChangeStatus`
  (params (InstigatedBy :type "Controller Object Reference"))
  (bind _returnvalue (`Controller.K2_GetPawn` InstigatedBy))
  (`self.UpdateText`)
  (bind _return (`/Game/Blueprints/BP_StatusComponent.IsDead` (`self.BP_StatusComponent`)))
  (if (not _return)
    (`/Engine/EditorBlueprintResources/StandardMacros.IsValid` InstigatedBy
      (:`Is Valid`
        (`/Engine/EditorBlueprintResources/StandardMacros.IsValid` _returnvalue
          (:`Is Valid`
            (set `self.AttackTarget` _returnvalue)
            (goto _label)))))))

(event `self.BP_StatusComponent.OnDeath`
  (`Controller.StopMovement` (`self.GetController`))
  (set `self.Behavior` "NewEnumerator3")
  (`PrimitiveComponent.SetCollisionEnabled` (`self.CapsuleComponent`) "NoCollision")
  (`/Game/Blueprints/BP_ItemDropComponent.DropItem` (`self.BP_ItemDropComponent`)))

(event `/Game/Blueprints/BPI_AnimNotifySendMessage.AnimNotifySendMessage`
  (params (Message :type Name))
  (switch `name` Message
    (:`DeathEnd`
      (`KismetSystemLibrary.Delay` 3.0)
      (`self.K2_DestroyActor`))
    (:`AttackTarget`
      (bind _return (`self.IsValidAttackTarget`))
      (if _return
        (`GameplayStatics.ApplyDamage` (`self.AttackTarget`) (`/Game/Blueprints/BP_StatusComponent.Damage` (`self.BP_StatusComponent`)) null self)))
    (:`AttackEnd`
      (bind _return_2 (`self.IsValidAttackTarget`))
      (if (not _return_2)
        (set `self.Behavior` "NewEnumerator0")))))

(event `self.BP_DataTableComponent.OnApplyMonsterInfo`
  (params (Info :type "/Game/Blueprints/MonsterStruct Structure"))
  (bind (_name _level) (break `/Game/Blueprints/MonsterStruct` Info))
  (set `self.Level` _level)
  (set `self.Name` (`KismetStringLibrary.Conv_NameToString` _name))
  (`/Game/Blueprints/BP_StatusComponent.SetDataByMonsterStruct` (`self.BP_StatusComponent`) Info)
  (`self.UpdateText`))

(fn `IsValidAttackTarget`
  (returns (Return :type Boolean))
  (`/Engine/EditorBlueprintResources/StandardMacros.IsValid` (`self.AttackTarget`)
    (:`Is Valid`
      (if (<= (`self.GetDistanceTo` (`self.AttackTarget`)) (`self.AttackDistance`))
        (return true)
        (else
          _)))
    (:`Is Not Valid`
      _))
  (return false))

(fn `UpdateText`
  (`TextRenderComponent.K2_SetText` (`self.TextRender`) (`KismetTextLibrary.Conv_StringToText` (`KismetStringLibrary.BuildString_Double` (`self.Name`) "[" (`/Game/Blueprints/BP_StatusComponent.HP` (`self.BP_StatusComponent`)) "]"))))

(fn `UserConstructionScript`)