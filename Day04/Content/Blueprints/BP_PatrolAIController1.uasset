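; AI controller for a patroller that runs BT_Patroller1 on BB_Patroller1 and reacts to AI Perception.
; Sight writes the visible player or last-seen location to the blackboard.
; With no player in sight, hearing maintains a HearingLocations array, flags ChangeNoiseLocation and stops movement when the newest noise is lost.
; Keys 1–3 print perception debug info; an older move-and-patrol graph remains disconnected.
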(event `self.ReceiveBeginPlay`
  (`self.UseBlackboard` "/Game/Blueprints/AI/BB_Patroller1.BB_Patroller1")
  (`self.RunBehaviorTree` "/Game/Blueprints/AI/BT_Patroller1.BT_Patroller1"))

(event `self.ReceiveTick`
  (params (DeltaSeconds :type "Float (single-precision)")))

(event `Key|One`
  (params (Key :type "Key Structure"))
  (:`Pressed`
    (bind (_info _returnvalue) (`AIPerceptionComponent.GetActorsPerception` (`self.AIPerception`) (`GameplayStatics.GetPlayerPawn` 0)))
    (if _returnvalue
      (bind (_target _lastsensedstimuli) (break `ActorPerceptionBlueprintInfo` _info))
      (for _array_element _lastsensedstimuli
        (bind _returnvalue_2 (`AIPerceptionSystem.GetSenseClassForStimulus` _array_element))
        (if (`KismetSystemLibrary.IsValidClass` _returnvalue_2)
          (bind (_age _expirationage _strength _stimuluslocation _receiverlocation _tag _bsuccessfullysensed) (break `AIStimulus` _array_element))
          (`KismetSystemLibrary.PrintString` (`KismetStringLibrary.Concat_StrStr` (`KismetStringLibrary.Conv_ObjectToString` _target) "[" (`KismetSystemLibrary.GetClassDisplayName` _returnvalue_2) "][" (`KismetStringLibrary.Conv_DoubleToString` _age) "][" (`KismetStringLibrary.Conv_DoubleToString` _expirationage) "][" (`KismetStringLibrary.Conv_BoolToString` _bsuccessfullysensed) "][")))))))

(event `Key|Two`
  (params (Key :type "Key Structure"))
  (:`Pressed`
    (for _array_element (`AIPerceptionComponent.GetCurrentlyPerceivedActors` (`self.AIPerception`) null)
      (`KismetSystemLibrary.PrintString` (`KismetSystemLibrary.GetDisplayName` _array_element)))))

(event `Key|Three`
  (params (Key :type "Key Structure"))
  (:`Pressed`
    (for _array_element (`AIPerceptionComponent.GetKnownPerceivedActors` (`self.AIPerception`) null)
      (`KismetSystemLibrary.PrintString` (`KismetSystemLibrary.GetDisplayName` _array_element)))))

(event `self.AIPerception.OnPerceptionUpdated`
  (params (UpdatedActors :type "Array of Actor Object Reference (by ref)")))

(event `self.AIPerception.OnTargetPerceptionUpdated`
  (params (Actor :type "Actor Object Reference") (Stimulus :type "AIStimulus Structure"))
  (bind _returnvalue (`AIPerceptionSystem.GetSenseClassForStimulus` Stimulus))
  (if (== _returnvalue "/Script/AIModule.AISense_Sight")
    (`self.ProcessAISense_Sight` Actor Stimulus)
    (elif (== _returnvalue "/Script/AIModule.AISense_Hearing")
      (`self.ProcessAISense_Hearing` Actor Stimulus))))

(fn `ProcessAISense_Hearing`
  (params (Actor :type "Actor Object Reference") (Stimulus :type "AIStimulus Structure"))
  (bind (_age _expirationage _strength _stimuluslocation _receiverlocation _tag _bsuccessfullysensed) (break `AIStimulus` Stimulus))
  (bind _hearinglocations (`self.HearingLocations`))
  (bind _returnvalue (`KismetArrayLibrary.Array_Length` _hearinglocations))
  (if (`KismetSystemLibrary.IsValid` (`self.PlayerInSight`))
    _
    (elif _bsuccessfullysensed
      (`KismetArrayLibrary.Array_Add` (`self.HearingLocations`) _stimuluslocation)
      (`BlackboardComponent.SetValueAsBool` (`self.Blackboard`) "ChangeNoiseLocation" true :!label _label)
      (elif (> _returnvalue 0)
        ;[1 1 1] Check last elemnt for moving or not
        (if (== (`|GetArrayItem` _hearinglocations (- _returnvalue 1)) _stimuluslocation)
          (`self.StopMovement`))
        (`KismetArrayLibrary.Array_RemoveItem` (`self.HearingLocations`) _stimuluslocation)
        (goto _label)))))

(fn `ProcessAISense_Sight`
  (params (Actor :type "Actor Object Reference") (Stimulus :type "AIStimulus Structure"))
  (bind (_age _expirationage _strength _stimuluslocation _receiverlocation _tag _bsuccessfullysensed) (break `AIStimulus` Stimulus))
  (if (== (`GameplayStatics.GetPlayerPawn` 0) Actor)
    (if _bsuccessfullysensed
      (set `self.PlayerInSight` (`GameplayStatics.GetPlayerPawn` 0))
      (set `self.LastPlayerLocation` (0.0 0.0 0.0))
      (`BlackboardComponent.SetValueAsObject` (`self.Blackboard`) "PlayerInSight" (`self.PlayerInSight`))
      (`BlackboardComponent.ClearValue` (`self.Blackboard`) "LastPlayerLocation")
      (else
        (set `self.PlayerInSight` null)
        (set `self.LastPlayerLocation` _stimuluslocation)
        (`BlackboardComponent.ClearValue` (`self.Blackboard`) "PlayerInSight")
        (`BlackboardComponent.SetValueAsVector` (`self.Blackboard`) "LastPlayerLocation" (`self.LastPlayerLocation`))))))

(fn `UserConstructionScript`)