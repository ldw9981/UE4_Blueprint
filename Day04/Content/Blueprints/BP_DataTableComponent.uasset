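; BP_DataTableComponent is a component that loads item and monster data from data tables on BeginPlay.
; ApplyDataTable checks each positive ID independently and converts it to a row name to look up in the item or monster table.
; A found row is broadcast through the OnApplyItemInfo or OnApplyMonsterInfo dispatcher, leaving its use to listeners.
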(event `self.ReceiveBeginPlay`
  (`self.ApplyDataTable`))

(fn `ApplyDataTable`
  (bind _monsterdatatableid (`self.MonsterDataTableID`))
  (bind _itemdatatableid (`self.ItemDataTableID`))
  (`|ExecutionSequence`
    (:`then_0`
      (if (> _itemdatatableid 0)
        (bind _returnvalue (`|GetDataTableRow` "/Game/Blueprints/ItemDataTable.ItemDataTable" (`KismetStringLibrary.Conv_StringToName` (`KismetStringLibrary.Conv_IntToString` _itemdatatableid)))
          (:`then`
            (`self.OnApplyItemInfo` _returnvalue)))))
    (:`then_1`
      (if (> _monsterdatatableid 0)
        (bind _returnvalue_2 (`|GetDataTableRow` "/Game/Blueprints/MonsterDataTable.MonsterDataTable" (`KismetStringLibrary.Conv_StringToName` (`KismetStringLibrary.Conv_IntToString` _monsterdatatableid)))
          (:`then`
            (`self.OnApplyMonsterInfo` _returnvalue_2)))))))