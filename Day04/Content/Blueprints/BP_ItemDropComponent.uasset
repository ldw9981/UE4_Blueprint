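; Actor component that drops one weighted-random item actor from a configurable drop list.
; BeginPlay sums the Probablity weights of ItemDropList into MaxProbablity.
; DropItem rolls a random integer below that total, walks cumulative weight ranges via IsInRange, and spawns the matching class at the owner's transform.
; An entry without a valid class yields no drop, and IsInRange's Length argument acts as an exclusive end bound.
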(event `self.ReceiveBeginPlay`
  (bind _itemdroplist (`self.ItemDropList`))
  (if (!= (`KismetArrayLibrary.Array_Length` _itemdroplist) 0)
    (for _array_element _itemdroplist
      (set `self.MaxProbablity` (+ (`self.MaxProbablity`) (`.Probablity_7_0AEF0DF04AC33135CE28628BE04A1595` (break `/Game/Blueprints/ItemDropPairStruct` _array_element)))))))

(fn `DropItem`
  (locals (PrevAccProbability :type Integer64) (RandomValue :type Integer64))
  (bind _itemdroplist (`self.ItemDropList`))
  (bind _prevaccprobability (`local.PrevAccProbability`))
  (if (!= (`KismetArrayLibrary.Array_Length` _itemdroplist) 0)
    (set `local.RandomValue` (`KismetMathLibrary.RandomInteger64` (`self.MaxProbablity`)))
    (for _array_element _itemdroplist
      (bind (_itemactor _probablity) (break `/Game/Blueprints/ItemDropPairStruct` _array_element))
      (bind _return (`self.IsInRange` _prevaccprobability (+ _prevaccprobability _probablity) (`local.RandomValue`)))
      (if _return
        (if (`KismetSystemLibrary.IsValidClass` _itemactor)
          (`|SpawnActorFromClass` _itemactor (`Actor.GetTransform` (`self.GetOwner`)) "Undefined" "OverrideRootScale" null null)
          (break)
          (else
            (break)))
        (else
          (set `local.PrevAccProbability` (+ (`local.PrevAccProbability`) _probablity)))))))

(fn `IsInRange`
  (params (Begin :type Integer64) (Length :type Integer64) (Value :type Integer64))
  (returns (Return :type Boolean))
  (return (and (<= Begin Value) (< Value Length))))