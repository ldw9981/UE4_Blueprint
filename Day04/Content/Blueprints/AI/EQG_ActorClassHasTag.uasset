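; An EQS generator that produces nearby actors of a given class carrying a specific tag as query items.
; It runs a sphere overlap around the first context location, filtered by radius, object types and actor class.
; Each overlapped actor that has the configured tag is added as a generated actor.
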(fn `DoItemGeneration`
  (params (ContextLocations :type "Array of Vector Structure (by ref)"))
  (bind _outactors (`KismetSystemLibrary.SphereOverlapActors` (`|GetArrayItem` ContextLocations) (`self.Radius`) (`self.ObjectTypes`) (`self.ActorClass`)))
  (for _array_element _outactors
    (if (`Actor.ActorHasTag` _array_element (`self.Tag`))
      (`self.AddGeneratedActor` _array_element)))
  (return))