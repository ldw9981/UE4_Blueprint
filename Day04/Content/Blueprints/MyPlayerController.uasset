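; Player controller Blueprint that opens an in-game pause menu when Tab is pressed.
; On a successful pause it creates and displays InGameMenuWidget, switches to UI-only input and shows the mouse cursor.
; It binds the widget's OnReturnToGame event to a custom event that removes the menu, restores game-only input, hides the cursor and unpauses.
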(event `self.ReceiveBeginPlay`)

(event `Key|Tab`
  (params (Key :type "Key Structure"))
  (bind _returnvalue (`GameplayStatics.GetPlayerController` 0))
  (:`Pressed`
    (bind _returnvalue_2 (`GameplayStatics.SetGamePaused` true))
    (if _returnvalue_2
      (bind _returnvalue_3 (`|CreateWidget` "/Game/Blueprints/UI/InGameMenuWidget.InGameMenuWidget_C" (`GameplayStatics.GetPlayerController` 0)))
      (set `self.NewVar_0` _returnvalue_3)
      (add `/Game/Blueprints/UI/InGameMenuWidget.OnReturnToGame` (`self.NewVar_0`) (delegate `커스텀이벤트_0`))
      (`UserWidget.AddToViewport` (`self.NewVar_0`) 0)
      (`WidgetBlueprintLibrary.SetInputMode_UIOnlyEx` _returnvalue null)
      (set `PlayerController.bShowMouseCursor` true _returnvalue))))

(event `커스텀이벤트_0`
  (bind _returnvalue (`GameplayStatics.GetPlayerController` 0))
  (`Widget.RemoveFromParent` (`self.NewVar_0`))
  (`WidgetBlueprintLibrary.SetInputMode_GameOnly` _returnvalue)
  (set `PlayerController.bShowMouseCursor` false _returnvalue)
  (`GameplayStatics.SetGamePaused` false))

(fn `UserConstructionScript`)