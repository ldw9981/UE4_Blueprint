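; BP_RandomSpawner spawns a set number of randomly chosen actor classes inside its Box at BeginPlay.
; Downward Visibility traces between random box points set spawn locations; only hits produce spawns.
; Spawned actors with a BP_DataTableComponent receive a random level within MinLevel and MaxLevel.
; With UseRespawn, destroyed actors increment a pending count, consumed after a delay to spawn replacements through the same path.
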(event `self.ReceiveBeginPlay`
  (bind _spawnactorclass (`self.SpawnActorClass`))
  (bind _box (`self.Box`))
  (bind _returnvalue (`KismetMathLibrary.RandomPointInBoundingBox` (`SceneComponent.K2_GetComponentLocation` _box) (`BoxComponent.GetUnscaledBoxExtent` _box)))
  (for _ (range (`self.Number`))
    (bind (_outhit _returnvalue_2) (`KismetSystemLibrary.LineTraceSingle` _returnvalue (+ _returnvalue (0.0 0.0 -999.0)) "TraceTypeQuery1" :!label _label))
    (if _returnvalue_2
      (bind _returnvalue_3 (`|SpawnActorFromClass` (`|GetArrayItem` _spawnactorclass (`KismetMathLibrary.RandomInteger` (`KismetArrayLibrary.Array_Length` _spawnactorclass))) (`KismetMathLibrary.MakeTransform` (`.Location` (`GameplayStatics.BreakHitResult` _outhit))) "AdjustIfPossibleButAlwaysSpawn" "OverrideRootScale" null null))
      (`/Engine/EditorBlueprintResources/StandardMacros.IsValid` _returnvalue_3
        (:`Is Valid`
          (`|ExecutionSequence`
            (:`then_0`
              (bind _returnvalue_4 (`self.GetComponentByClass` _returnvalue_3 "/Game/Blueprints/BP_DataTableComponent.BP_DataTableComponent_C"))
              (`/Engine/EditorBlueprintResources/StandardMacros.IsValid` _returnvalue_4
                (:`Is Valid`
                  (`/Game/Blueprints/BP_DataTableComponent.ApplyDataTable` _returnvalue_4 (- (`KismetMathLibrary.RandomIntegerInRange` (`self.MinLevel`) (`self.MaxLevel`)) 1)))))
            (:`then_1`
              (if (`self.UseRespawn`)
                (add `self.OnDestroyed` _returnvalue_3 (delegate `OnDestroyed_Event_0`))
                (`KismetSystemLibrary.Delay` (`self.RespawnDelayTime`) :!label _label_2)
                (if (> (`self.RespawnCount`) 0)
                  (`/Engine/EditorBlueprintResources/StandardMacros.DecrementInt` (`self.RespawnCount`)
                    (:`  `
                      (goto _label))))))))))))

(event `OnDestroyed_Event_0` :!signature `self.OnDestroyed`
  (params (DestroyedActor :type "Actor Object Reference"))
  (`/Engine/EditorBlueprintResources/StandardMacros.IncrementInt` (`self.RespawnCount`)
    (:`  `
      (goto _label_2))))

(fn `UserConstructionScript`)