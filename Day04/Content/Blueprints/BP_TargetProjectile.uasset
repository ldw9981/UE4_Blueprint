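; Homing projectile that chases a target actor and damages what it hits.
; Each tick it rotates toward the TargetActor set through SetTargetActor and redirects ProjectileMovement velocity along that facing at unchanged speed, or destroys itself if the target is invalid.
; A Sphere hit applies Damage, supplied by BP_DataTableComponent's item info, to the hit actor and destroys the projectile.
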(event `self.ReceiveBeginPlay`)

(event `self.ReceiveTick`
  (params (DeltaSeconds :type "Float (single-precision)"))
  (bind (_returnvalue_roll _returnvalue_pitch _returnvalue_yaw) (`KismetMathLibrary.BreakRotator` (`self.K2_GetActorRotation`)))
  (bind _projectilemovement (`self.ProjectileMovement`))
  (`/Engine/EditorBlueprintResources/StandardMacros.IsValid` (`self.TargetActor`)
    (:`Is Valid`
      (`self.K2_SetActorRotation` (`KismetMathLibrary.FindLookAtRotation` (`self.K2_GetActorLocation`) (`self.K2_GetActorLocation` (`self.TargetActor`))))
      (set `MovementComponent.Velocity` (`KismetMathLibrary.CreateVectorFromYawPitch` _returnvalue_yaw _returnvalue_pitch (`KismetMathLibrary.VSize` (`MovementComponent.Velocity` _projectilemovement))) _projectilemovement))
    (:`Is Not Valid`
      (`self.K2_DestroyActor`))))

(event `self.Sphere.OnComponentHit`
  (params (HitComponent :type "PrimitiveComponent Object Reference") (OtherActor :type "Actor Object Reference") (OtherComp :type "PrimitiveComponent Object Reference") (NormalImpulse :type "Vector Structure") (Hit :type "HitResult Structure (by ref)"))
  (`GameplayStatics.ApplyDamage` OtherActor (`self.Damage`) (`self.GetInstigatorController`) self)
  (`self.K2_DestroyActor`))

(event `self.BP_DataTableComponent.OnApplyItemInfo`
  (params (Info :type "/Game/Blueprints/ItemStruct Structure"))
  (set `self.Damage` (`.Damage_6_CE4510E4466D8211B2339E83CF85C58B` (break `/Game/Blueprints/ItemStruct` Info))))

(fn `SetTargetActor`
  (params (TargetActor :type "Actor Object Reference"))
  (set `self.TargetActor` TargetActor))

(fn `UserConstructionScript`)