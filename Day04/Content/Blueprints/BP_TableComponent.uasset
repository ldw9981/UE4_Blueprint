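; BP_TableComponent is a component that fetches level-based monster and item data and broadcasts it.
; ApplyTable takes a level, caps it at each type's max level and offsets it from that type's base ID to form a DataTable row name.
; Rows found in MonsterTable and ItemTable fire OnApplyMonsterInfo and OnApplyItemInfo with the row and the requested level.
; Either lookup is skipped when its base ID or max level is not positive.
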(fn `ApplyTable`
  (params (Level :type Integer))
  (bind _monsterbasetableid (`self.MonsterBaseTableID`))
  (bind _itembasetableid (`self.ItemBaseTableID`))
  (`|ExecutionSequence`
    (:`then_0`
      (if (and (> _monsterbasetableid 0) (> (`self.MonsterMaxLevel`) 0))
        (bind _returnvalue (`|GetDataTableRow` "/Game/Blueprints/MonsterTable.MonsterTable" (`KismetStringLibrary.Conv_StringToName` (`KismetStringLibrary.Conv_IntToString` (+ (- _monsterbasetableid 1) (`KismetMathLibrary.Min` (`self.MonsterMaxLevel`) Level)))))
          (:`then`
            (`self.OnApplyMonsterInfo` _returnvalue Level)))))
    (:`then_1`
      (if (and (> _itembasetableid 0) (> (`self.ItemMaxLevel`) 0))
        (bind _returnvalue_2 (`|GetDataTableRow` "/Game/Blueprints/ItemTable.ItemTable" (`KismetStringLibrary.Conv_StringToName` (`KismetStringLibrary.Conv_IntToString` (+ (- _itembasetableid 1) (`KismetMathLibrary.Min` (`self.ItemMaxLevel`) Level)))))
          (:`then`
            (`self.OnApplyItemInfo` _returnvalue_2 Level)))))))