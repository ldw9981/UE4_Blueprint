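; BP_Barrel is a destructible barrel that shows its HP on a text render and awards score when destroyed.
; A status component drives it: status changes refresh the HP text, and its death event destroys the actor.
; On destruction, the barrel applies small radial damage around its location and adds points through the custom game instance.
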(event `self.ReceiveBeginPlay`
  (`TextRenderComponent.K2_SetText` (`self.TextRender`) (`KismetTextLibrary.Conv_DoubleToText` (`self.HP`) "HalfToEven")))

(event `self.ReceiveDestroyed`
  (`GameplayStatics.ApplyRadialDamage` :`BaseDamage` 10.0 :`Origin` (`self.K2_GetActorLocation`) :`DamageRadius` 100.0 :`DamageCauser` self :`InstigatedByController` null)
  (bind _asmy_game_instance (cast `/Game/Blueprints/MyGameInstance` (`GameplayStatics.GetGameInstance`)))
  (`/Game/Blueprints/MyGameInstance.AddScore` _asmy_game_instance 100))

(event `self.BP_StatusComponent.OnDeath`
  (`self.K2_DestroyActor`))

(event `self.BP_StatusComponent.OnChangeStatus`
  (`TextRenderComponent.K2_SetText` (`self.TextRender`) (`KismetTextLibrary.Conv_DoubleToText` (`/Game/Blueprints/BP_StatusComponent.HP` (`self.BP_StatusComponent`)) "HalfToEven")))

(fn `UserConstructionScript`)