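; Target spawner that, on BeginPlay, spawns a random actor class at each attached marker actor of the target class inside its box.
; Spawned actors with a BP_DataTableComponent get a random level from the configured range applied.
; With respawn enabled, destroyed actors queue their locations, and a shared Delay pops the oldest one on completion, looping back into the same spawn logic.
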(event `self.ReceiveBeginPlay`
  (bind _spawnactorclass (`self.SpawnActorClass`))
  (bind _requestlocation (`self.RequestLocation`))
  (bind _box (`self.Box`))
  (for _array_element (`self.GetAttachedActors` true)
    (if (== (`self.TargetActorClass`) (`GameplayStatics.GetObjectClass` _array_element))
      (bind _returnvalue (`self.K2_GetActorLocation` _array_element))
      (if (`KismetMathLibrary.IsPointInBox` _returnvalue (`SceneComponent.K2_GetComponentLocation` _box) (`BoxComponent.BoxExtent` _box))
        (set `self.SpawnLocation` _returnvalue)
        (bind _returnvalue_2 (`|SpawnActorFromClass` (`|GetArrayItem` _spawnactorclass (`KismetMathLibrary.RandomInteger` (`KismetArrayLibrary.Array_Length` _spawnactorclass))) (`KismetMathLibrary.MakeTransform` (`self.SpawnLocation`)) "Undefined" "OverrideRootScale" null null :!label _label))
        (`/Engine/EditorBlueprintResources/StandardMacros.IsValid` _returnvalue_2
          (:`Is Valid`
            (`|ExecutionSequence`
              (:`then_0`
                (bind _returnvalue_3 (`self.GetComponentByClass` _returnvalue_2 "/Game/Blueprints/BP_DataTableComponent.BP_DataTableComponent_C"))
                (`/Engine/EditorBlueprintResources/StandardMacros.IsValid` _returnvalue_3
                  (:`Is Valid`
                    (`/Game/Blueprints/BP_DataTableComponent.ApplyDataTable` _returnvalue_3 (- (`KismetMathLibrary.RandomIntegerInRange` (`self.MinLevel`) (`self.MaxLevel`)) 1)))))
              (:`then_1`
                (if (`self.UseRespawn`)
                  (add `self.OnDestroyed` _returnvalue_2 (delegate `OnDestroyed_Event_0`))
                  (`KismetSystemLibrary.Delay` (`self.RespawnDelay`) :!label _label_2)
                  (if (> (`KismetArrayLibrary.Array_Length` _requestlocation) 0)
                    (set `self.SpawnLocation` (`|GetArrayItem` _requestlocation))
                    (`KismetArrayLibrary.Array_Remove` _requestlocation)
                    (goto _label)))))))))))

(event `OnDestroyed_Event_0` :!signature `self.OnDestroyed`
  (params (DestroyedActor :type "Actor Object Reference"))
  (`KismetArrayLibrary.Array_Add` (`self.RequestLocation`) (`self.K2_GetActorLocation` DestroyedActor))
  (goto _label_2))

(fn `UserConstructionScript`)