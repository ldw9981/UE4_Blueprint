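; AI controller for a player follower pawn, running the BT_PlayerFollower behavior tree on the BB_PlayerFollower blackboard.
; Mirrors the pawn's HP percent from BP_StatusComponent into the blackboard and stops the brain on death.
; Sight perception keeps a count of visible Enemy-tagged actors in the blackboard.
; Hearing (noise location) and damage (debug print) handlers exist but are not wired to perception updates.
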(event `self.ReceiveBeginPlay`
  (bind _returnvalue (`self.GetComponentByClass` (`self.K2_GetPawn`) "/Game/Blueprints/BP_StatusComponent.BP_StatusComponent_C"))
  (`self.UseBlackboard` "/Game/Blueprints/AI/BB_PlayerFollower.BB_PlayerFollower")
  (`self.RunBehaviorTree` "/Game/Blueprints/AI/BT_PlayerFollower.BT_PlayerFollower")
  (add `/Game/Blueprints/BP_StatusComponent.OnChangeStatus` _returnvalue (delegate `커스텀이벤트_0`))
  (bind _return (`/Game/Blueprints/BP_StatusComponent.GetPercentHP` _returnvalue))
  (`BlackboardComponent.SetValueAsFloat` (`self.Blackboard`) "PercentHP" _return)
  (add `/Game/Blueprints/BP_StatusComponent.OnDeath` _returnvalue (delegate `OnDeath_Event_0`)))

(event `OnDeath_Event_0`
  (`BrainComponent.StopLogic` (`self.BrainComponent`) "Death"))

(event `커스텀이벤트_0`
  (params (InstigatedBy :type "Controller Object Reference") (PercentHP :type "Float (double-precision)"))
  (`BlackboardComponent.SetValueAsFloat` (`self.Blackboard`) "PercentHP" PercentHP))

(event `self.ReceiveTick`
  (params (DeltaSeconds :type "Float (single-precision)")))

(event `self.AIPerception.OnTargetPerceptionUpdated`
  (params (Actor :type "Actor Object Reference") (Stimulus :type "AIStimulus Structure"))
  (bind _returnvalue (`AIPerceptionSystem.GetSenseClassForStimulus` Stimulus))
  (if (== _returnvalue "/Script/AIModule.AISense_Sight")
    (`self.ProcessAISense_Sight` Actor Stimulus)
    (elif (== _returnvalue "/Script/AIModule.AISense_Hearing")
      _
      (elif (== _returnvalue "/Script/AIModule.AISense_Damage")
        _))))

(fn `ProcessAISense_Damage`
  (params (Actor :type "Actor Object Reference") (Stimulus :type "AIStimulus Structure"))
  (`KismetSystemLibrary.PrintString` (`KismetStringLibrary.Conv_BoolToString` (`.bSuccessfullySensed` (break `AIStimulus` Stimulus)))))

(fn `ProcessAISense_Hearing`
  (params (Actor :type "Actor Object Reference") (Stimulus :type "AIStimulus Structure"))
  (bind (_age _expirationage _strength _stimuluslocation _receiverlocation _tag _bsuccessfullysensed) (break `AIStimulus` Stimulus))
  (if (`KismetSystemLibrary.IsValid` null)
    _
    (elif _bsuccessfullysensed
      (`KismetArrayLibrary.Array_Add` (`self.HearingLocations`) _stimuluslocation)
      (`BlackboardComponent.SetValueAsVector` (`self.Blackboard`) "NoiseLocation" _stimuluslocation)
      (else
        (`KismetArrayLibrary.Array_RemoveItem` (`self.HearingLocations`) _stimuluslocation)))))

(fn `ProcessAISense_Sight`
  (params (Actor :type "Actor Object Reference") (Stimulus :type "AIStimulus Structure"))
  (bind _numenermyinsight (`self.NumEnermyInSight`))
  (if (`self.ActorHasTag` Actor "Enemy")
    (if (`.bSuccessfullySensed` (break `AIStimulus` Stimulus))
      (`/Engine/EditorBlueprintResources/StandardMacros.IncrementInt` _numenermyinsight
        (:`  `
          _))
      (else
        (`/Engine/EditorBlueprintResources/StandardMacros.DecrementInt` _numenermyinsight
          (:`  `
            _))))
    (`BlackboardComponent.SetValueAsInt` (`self.Blackboard`) "NumEnemyInSight" (`self.NumEnermyInSight`))))

(fn `UserConstructionScript`)