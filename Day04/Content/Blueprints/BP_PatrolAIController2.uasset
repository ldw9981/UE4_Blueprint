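; AI controller for the BP_Patrol2 pawn that runs its patrol behavior tree and feeds the blackboard.
; On BeginPlay it binds to the pawn's status component, mirroring health percent into the blackboard and stopping brain logic on death.
; Sight perception tracks the player pawn, storing either the visible player or the last seen location.
; Hearing records noise locations and publishes the newest to the blackboard only while no player is in sight.
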(event `self.ReceiveBeginPlay`
  (`self.UseBlackboard` "/Game/Blueprints/AI/BB_Patrol2.BB_Patrol2")
  (`self.RunBehaviorTree` "/Game/Blueprints/AI/BT_Patrol2.BT_Patrol2")
  (bind _asbp_patrol_2 (cast `/Game/Blueprints/BP_Patrol2` (`self.K2_GetPawn`)))
  (bind _returnvalue (`self.GetComponentByClass` _asbp_patrol_2 "/Game/Blueprints/BP_StatusComponent.BP_StatusComponent_C"))
  (add `/Game/Blueprints/BP_StatusComponent.OnChangeStatus` _returnvalue (delegate `커스텀이벤트_0`))
  (bind _return (`/Game/Blueprints/BP_StatusComponent.GetPercentHP` _returnvalue))
  (`BlackboardComponent.SetValueAsFloat` (`self.Blackboard`) "PercentHP" _return)
  (add `/Game/Blueprints/BP_StatusComponent.OnDeath` _returnvalue (delegate `OnDeath_Event_0`)))

(event `OnDeath_Event_0`
  (`BrainComponent.StopLogic` (`self.BrainComponent`) "Death"))

(event `커스텀이벤트_0`
  (params (InstigatedBy :type "Controller Object Reference") (PercentHP :type "Float (double-precision)"))
  (`BlackboardComponent.SetValueAsFloat` (`self.Blackboard`) "PercentHP" PercentHP))

(event `self.ReceiveTick`
  (params (DeltaSeconds :type "Float (single-precision)")))

(event `self.AIPerception.OnTargetPerceptionUpdated`
  (params (Actor :type "Actor Object Reference") (Stimulus :type "AIStimulus Structure"))
  (bind _returnvalue (`AIPerceptionSystem.GetSenseClassForStimulus` Stimulus))
  (if (== _returnvalue "/Script/AIModule.AISense_Sight")
    (`self.ProcessAISense_Sight` Actor Stimulus)
    (elif (== _returnvalue "/Script/AIModule.AISense_Hearing")
      (`self.ProcessAISense_Hearing` Actor Stimulus))))

(fn `ProcessAISense_Hearing`
  (params (Actor :type "Actor Object Reference") (Stimulus :type "AIStimulus Structure"))
  (bind (_age _expirationage _strength _stimuluslocation _receiverlocation _tag _bsuccessfullysensed) (break `AIStimulus` Stimulus))
  (if (`KismetSystemLibrary.IsValid` (`self.PlayerInSight`))
    _
    (elif _bsuccessfullysensed
      (`KismetArrayLibrary.Array_Add` (`self.HearingLocations`) _stimuluslocation)
      (`BlackboardComponent.SetValueAsVector` (`self.Blackboard`) "NoiseLocation" _stimuluslocation)
      (else
        (`KismetArrayLibrary.Array_RemoveItem` (`self.HearingLocations`) _stimuluslocation)))))

(fn `ProcessAISense_Sight`
  (params (Actor :type "Actor Object Reference") (Stimulus :type "AIStimulus Structure"))
  (bind (_age _expirationage _strength _stimuluslocation _receiverlocation _tag _bsuccessfullysensed) (break `AIStimulus` Stimulus))
  (if (== (`GameplayStatics.GetPlayerPawn` 0) Actor)
    (if _bsuccessfullysensed
      (set `self.PlayerInSight` (`GameplayStatics.GetPlayerPawn` 0))
      (set `self.LastPlayerLocation` (0.0 0.0 0.0))
      (`BlackboardComponent.SetValueAsObject` (`self.Blackboard`) "PlayerInSight" (`self.PlayerInSight`))
      (`BlackboardComponent.ClearValue` (`self.Blackboard`) "LastPlayerLocation")
      (else
        (set `self.PlayerInSight` null)
        (set `self.LastPlayerLocation` _stimuluslocation)
        (`BlackboardComponent.ClearValue` (`self.Blackboard`) "PlayerInSight")
        (`BlackboardComponent.SetValueAsVector` (`self.Blackboard`) "LastPlayerLocation" (`self.LastPlayerLocation`))))))

(fn `UserConstructionScript`)