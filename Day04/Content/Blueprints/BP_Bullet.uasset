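; Bullet actor that damages whatever its collision sphere hits, then destroys itself.
; On BeginPlay it reads Damage from ItemTable, using a row name computed from BaseItemTableID and ItemLevel, if the ID is non-zero and the level is within ItemLevelMax.
; UpdateLevel does not increment the level: it sets ItemLevel to the lesser of ItemLevelMax and zero, and does not refresh Damage.
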(event `self.ReceiveBeginPlay`
  (if (and (!= (`self.BaseItemTableID`) 0) (<= (`self.ItemLevel`) (`self.ItemLevelMax`)))
    (bind _returnvalue (`|GetDataTableRow` "/Game/Blueprints/ItemTable.ItemTable" (`KismetStringLibrary.Conv_StringToName` (`KismetStringLibrary.Conv_IntToString` (+ (- (`self.BaseItemTableID`) 1) (`self.ItemLevel`)))))
      (:`then`
        (set `self.Damage` (`.Damage_6_CE4510E4466D8211B2339E83CF85C58B` (break `/Game/Blueprints/ItemStruct` _returnvalue)))))))

(event `self.Sphere.OnComponentHit`
  (params (HitComponent :type "PrimitiveComponent Object Reference") (OtherActor :type "Actor Object Reference") (OtherComp :type "PrimitiveComponent Object Reference") (NormalImpulse :type "Vector Structure") (Hit :type "HitResult Structure (by ref)"))
  (`GameplayStatics.ApplyDamage` OtherActor (`self.Damage`) null self)
  (`self.K2_DestroyActor`))

(event `/Game/Blueprints/BPI_Update.UpdateLevel`
  (params (Value :type Integer))
  (set `self.ItemLevel` (`KismetMathLibrary.Min` (`self.ItemLevelMax`))))

(fn `UserConstructionScript`)