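; BP_Patroller is an actor Blueprint that supplies patrol locations from its PatrolPoints list.
; GetNextPatrolLocation advances PatrolIndex with modulo wraparound, skipping invalid points by looping back, with no exit if all are invalid.
; GetCurrPatrolLocation returns the location at the current index without a validity check, and both return a default location when the list is empty.
; It contains no movement logic, and its event graph and construction script are empty.
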(fn `GetCurrPatrolLocation`
  (returns (Return :type "Vector Structure"))
  (locals (LocalReturnLocation :type "Vector Structure"))
  (if (!= (`KismetArrayLibrary.Array_Length` (`self.PatrolPoints`)) 0)
    (set `local.LocalReturnLocation` (`self.K2_GetActorLocation` (`|GetArrayItem` (`self.PatrolPoints`) (`self.PatrolIndex`)))))
  (return (`local.LocalReturnLocation`)))

(fn `GetNextPatrolLocation`
  (returns (Return :type "Vector Structure"))
  (locals (LocalReturnLocation :type "Vector Structure"))
  (bind _returnvalue (`KismetArrayLibrary.Array_Length` (`self.PatrolPoints`)))
  (if (!= _returnvalue 0)
    (bind _result (`/Engine/EditorBlueprintResources/StandardMacros.IncrementInt` (`self.PatrolIndex`) :!label _label)
      (:`  `
        (bind _output_get (set `self.PatrolIndex` (mod _result _returnvalue)))
        (if (< _output_get (`KismetArrayLibrary.Array_Length` (`self.PatrolPoints`)))
          (bind _output (`|GetArrayItem` (`self.PatrolPoints`) _output_get))
          (`/Engine/EditorBlueprintResources/StandardMacros.IsValid` _output
            (:`Is Valid`
              (set `local.LocalReturnLocation` (`self.K2_GetActorLocation` _output))
              (return (`local.LocalReturnLocation`)))
            (:`Is Not Valid`
              (goto _label))))))
    (else
      (return (`local.LocalReturnLocation`)))))

(fn `UserConstructionScript`)