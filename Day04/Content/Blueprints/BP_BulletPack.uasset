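; BP_BulletPack is an ammo pickup actor that gives bullets to the player and then destroys itself.
; On BeginPlay its table component applies data for its Level, and the returned item info sets the bullet count from Quantity and the floating text from Name.
; When the player's controlled pawn overlaps the sphere, it is cast to ThirdPersonCharacter and receives the bullets through AddBullet.
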(event `self.ReceiveBeginPlay`
  (`/Game/Blueprints/BP_TableComponent.ApplyTable` (`self.BP_TableComponent`) (`self.Level`)))

(event `self.Sphere.OnComponentBeginOverlap`
  (params (OverlappedComponent :type "PrimitiveComponent Object Reference") (OtherActor :type "Actor Object Reference") (OtherComp :type "PrimitiveComponent Object Reference") (OtherBodyIndex :type Integer) (bFromSweep :type Boolean) (SweepResult :type "HitResult Structure (by ref)"))
  (bind _returnvalue (`Controller.K2_GetPawn` (`GameplayStatics.GetPlayerController` 0)))
  (if (== OtherActor _returnvalue)
    (bind _asthird_person_character (cast `/Game/ThirdPersonBP/Blueprints/ThirdPersonCharacter` _returnvalue))
    (`/Game/ThirdPersonBP/Blueprints/ThirdPersonCharacter.Add Bullet` _asthird_person_character (`self.BulletNumber`))
    (`self.K2_DestroyActor`)))

(event `self.BP_TableComponent.OnApplyItemInfo`
  (params (Info :type "/Game/Blueprints/ItemStruct Structure") (Level :type Integer))
  (bind (_name _damage _quantity) (break `/Game/Blueprints/ItemStruct` Info))
  (set `self.Level` Level)
  (set `self.BulletNumber` (`KismetMathLibrary.FTrunc` _quantity))
  (`TextRenderComponent.K2_SetText` (`self.TextRender`) (`KismetTextLibrary.Conv_NameToText` _name)))

(fn `UserConstructionScript`)