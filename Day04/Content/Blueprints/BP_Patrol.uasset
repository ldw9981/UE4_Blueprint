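; BP_Patrol is a patrol route holder that supplies world locations from an array of patrol point actors.
; GetNextPatrolLocation increments PatrolIndex, wraps it with modulo to loop the route, and returns that point's location, without guarding against an empty array.
; GetCurrPatrolLocation returns the current point's location, or the local default when the array is empty.
; The event graph and construction script contain no logic.
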(fn `GetCurrPatrolLocation`
  (returns (Return :type "Vector Structure"))
  (locals (LocalReturnLocation :type "Vector Structure"))
  (if (!= (`KismetArrayLibrary.Array_Length` (`self.PatrolPoints`)) 0)
    (set `local.LocalReturnLocation` (`self.K2_GetActorLocation` (`|GetArrayItem` (`self.PatrolPoints`) (`self.PatrolIndex`)))))
  (return (`local.LocalReturnLocation`)))

(fn `GetNextPatrolLocation`
  (returns (Return :type "Vector Structure"))
  (bind _result (`/Engine/EditorBlueprintResources/StandardMacros.IncrementInt` (`self.PatrolIndex`))
    (:`  `
      (bind _output_get (set `self.PatrolIndex` (mod _result (`KismetArrayLibrary.Array_Length` (`self.PatrolPoints`)))))
      (return (`self.K2_GetActorLocation` (`|GetArrayItem` (`self.PatrolPoints`) _output_get))))))

(fn `UserConstructionScript`)