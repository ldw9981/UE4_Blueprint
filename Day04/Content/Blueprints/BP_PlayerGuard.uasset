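; BP_PlayerGuard is an AI guard character that attacks targets and provides patrol locations.
; On begin play it hands its status component to its widget for display.
; Animation notify messages drive combat: one applies status-based damage to the Blackboard's attack target with a forward knockback impulse, another destroys the guard shortly after death.
; Helper functions return the current patrol point or cycle through the patrol list.
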(event `self.ReceiveBeginPlay`
  (bind _asstatus_widget (cast `/Game/Blueprints/UI/StatusWidget` (`WidgetComponent.GetUserWidgetObject` (`self.Widget`))))
  (set `/Game/Blueprints/UI/StatusWidget.StatusComponent` (`self.BP_StatusComponent`) _asstatus_widget))

(event `/Game/Blueprints/BPI_AnimNotifySendMessage.AnimNotifySendMessage`
  (params (Message :type Name))
  (switch `name` Message
    (:`DeathEnd`
      (`KismetSystemLibrary.Delay` 1.0)
      (`self.K2_DestroyActor`))
    (:`TargetAttack`
      (bind _asactor (cast `Actor` (`BlackboardComponent.GetValueAsObject` (`AIBlueprintHelperLibrary.GetBlackboard` null) "AttackTargetActor")))
      (`GameplayStatics.ApplyDamage` _asactor (`/Game/Blueprints/BP_StatusComponent.Damage` (`self.BP_StatusComponent`)) (`self.GetController`) self)
      (bind _returnvalue (`self.GetComponentByClass` _asactor "/Script/Engine.CharacterMovementComponent"))
      (`/Engine/EditorBlueprintResources/StandardMacros.IsValid` _returnvalue
        (:`Is Valid`
          (`CharacterMovementComponent.AddImpulse` _returnvalue (* (`self.GetActorForwardVector`) 3000.0) true))))))

(fn `GetCurrPatrolLocation`
  (returns (Return :type "Vector Structure"))
  (locals (LocalReturnLocation :type "Vector Structure"))
  (if (!= (`KismetArrayLibrary.Array_Length` (`self.PatrolPoints`)) 0)
    (set `local.LocalReturnLocation` (`self.K2_GetActorLocation` (`|GetArrayItem` (`self.PatrolPoints`) (`self.PatrolIndex`)))))
  (return (`local.LocalReturnLocation`)))

(fn `GetNextPatrolLocation`
  (returns (Return :type "Vector Structure"))
  (bind _result (`/Engine/EditorBlueprintResources/StandardMacros.IncrementInt` (`self.PatrolIndex`))
    (:`  `
      (bind _output_get (set `self.PatrolIndex` (mod _result (`KismetArrayLibrary.Array_Length` (`self.PatrolPoints`)))))
      (return (`self.K2_GetActorLocation` (`|GetArrayItem` (`self.PatrolPoints`) _output_get))))))

(fn `UserConstructionScript`)